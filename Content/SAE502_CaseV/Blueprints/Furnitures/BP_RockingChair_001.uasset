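; Rocking chair furniture actor that starts a rocking animation with creaking sounds on BeginPlay.
; The Balancement timeline drives the mesh's roll from its Angle track and derives a proportional Y offset from the same value, so the chair shifts as it tilts.
; The timeline's Sons event track triggers a FlipFlop that alternates in and out creak sounds on the AudioGrincement component.
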(event Custom|LancerBalancement
  (bind _angle (Timeline|Balancement Play)
    (:Update
      (Transformation|SetRelativeRotation (Variables|Default|GetMesh) (Math|Rotator|MakeRotator _angle 0.0 0.0) false false)
      (Transformation|SetRelativeLocation (Variables|Default|GetMesh) (Math|Vector|MakeVector 0.0 (* _angle 0.8) 0.0) false false))
    (:Sons
      (Utilities|FlowControl|FlipFlop
        (:A
          (Audio|Components|Audio|SetSound (Variables|Default|GetAudio_grincement) "/Game/SAE502_CaseV/Audio/SFX/ROKCING_CHAIR/MS_ROCKING_CHAIR_IN.MS_ROCKING_CHAIR_IN")
          (Audio|Components|Audio|Play (Variables|Default|GetAudio_grincement) 0.0))
        (:B
          (Audio|Components|Audio|SetSound (Variables|Default|GetAudio_grincement) "/Game/SAE502_CaseV/Audio/SFX/ROKCING_CHAIR/MS_ROCKING_CHAIR_OUT.MS_ROCKING_CHAIR_OUT")
          (Audio|Components|Audio|Play (Variables|Default|GetAudio_grincement) 0.0))))))

(event EventBeginPlay
  (CallFunction|LancerBalancement))

(fn ConstructionScript)