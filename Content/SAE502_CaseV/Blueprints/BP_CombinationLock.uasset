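; Three-dial combination padlock puzzle: interacting blends the view to the lock's camera and moves input to it, and A exits.
; Z/S move an arrow selector between dials, while D/Q change the selected value modulo 10 and play a 36-degree timeline rotation, with a Busy flag blocking overlapping input.
; When values match CorrectCombination, it calls OnCadenasOuvert, opens, drops with physics, returns control and destroys itself.
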(event Custom|RotateDials
  (params (Forward? :type Boolean))
  (bind _returnvalue (Transformation|GetActorLocation))
  (bind _returnvalue_2 (Math|Random|RandomFloatinRange 0.95 1.05))
  (bind _returnvalue_3 (Math|Float|SelectFloat 36.0 -36.0 Forward?))
  (bind _dialsrotations (Variables|Default|GetDialsRotations))
  (bind _index (Variables|Default|GetIndex))
  (bind _output (Utilities|Array|Get(acopy) _dialsrotations _index))
  (bind _returnvalue_4 (+ _output _returnvalue_3))
  ;[0.15 0.15 0.15 0.5] Rotate Dial
  (if Forward?
    (Audio|PlaySoundatLocation "/Game/SAE502_CaseV/Audio/SFX/PadLock/Dial_01.Dial_01" _returnvalue "0, 0, 0" 1.0 _returnvalue_2 0.0 0 0 0 0)
    (bind _rotatedialz (Timeline|RotateDial PlayFromStart)
      (:Update
        (Transformation|SetRelativeRotation (Utilities|Array|Get(acopy) (Variables|Default|GetDials) (Variables|Default|GetIndex)) (Math|Rotator|MakeRotator 0.0 0.0 (Math|Float|Lerp _output _returnvalue_4 _rotatedialz)) false false))
      (:Finished
        (Utilities|Array|SetArrayElem (Variables|Default|GetDialsRotations) (Variables|Default|GetIndex) (Math|Float|%(Float) (+ (Math|Float|%(Float) _returnvalue_4 3.6e+02) 3.6e+02) 3.6e+02))
        (if (Utilities|Array|Identical (Variables|Default|GetCorrectCombination) (Variables|Default|GetDialsValue))
          (Default|CallOnCadenasOuvert)
          ;[0.15 0.15 0.15 0.5] Simple Lock Unlock Logic
          (Audio|PlaySoundatLocation "/Game/SAE502_CaseV/Audio/SFX/PadLock/Unlock.Unlock" (Transformation|GetActorLocation) "0, 0, 0" 1.0 1.0 0.0 0 0 0 0)
          (Transformation|SetRelativeRotation (Variables|Default|GetLockPiece) (Math|Rotator|MakeRotator -1e+01 0.0 29.0) false false)
          (Utilities|FlowControl|Delay 0.2)
          (Physics|SetSimulatePhysics (Variables|Default|GetLockBase) true)
          (CallFunction|Exit)
          (Utilities|FlowControl|Delay 4.0)
          (Actor|DestroyActor)
          (else
            (Variables|Default|SetBusy false)))))
    (else
      (Audio|PlaySoundatLocation "/Game/SAE502_CaseV/Audio/SFX/PadLock/Dial_Reverse.Dial_Reverse" _returnvalue "0, 0, 0" 1.0 _returnvalue_2 0.0 0 0 0 0)
      (Timeline|RotateDial PlayFromStart))))

(event Custom|Exit
  (bind _returnvalue (Game|GetPlayerController 0))
  ;[0.15 0.15 0.15 0.5] Exit From Puzzle Logic
  ;;[0.15 0.15 0.15 0.5] Cast to the player to get camera
  (bind _asbp_first_person_character (Utilities|Casting|CastToBP_FirstPersonCharacter (Game|GetPlayerCharacter 0)))
  (Game|Player|SetViewTargetwithBlend _returnvalue (Components|GetOwner (Variables|/Game/FirstPerson/Blueprints/BP_FirstPersonCharacter.BP_FirstPersonCharacter_C|GetFirstPersonCamera _asbp_first_person_character)) 0.4 "VTBlend_Linear" 0.0 false)
  (Input|DisableInput _returnvalue)
  (Input|EnableInput (Game|GetPlayerCharacter 0) _returnvalue))

(event Custom|UpdateSelectorPosition
  (Transformation|SetWorldLocation (Variables|Default|GetArrowsWidget) (Transformation|GetWorldLocation (Utilities|Array|Get(acopy) (Variables|Default|GetDialsAnchors) (Variables|Default|GetIndex))) false false))

(event EventBeginPlay
  (Variables|Default|SetDials (Utilities|Array|MakeArray (Variables|Default|GetDialTop) (Variables|Default|GetDialMid) (Variables|Default|GetDialBot)))
  (Variables|Default|SetDialsAnchors (Utilities|Array|MakeArray (Variables|Default|GetArrowTop) (Variables|Default|GetArrowMid) (Variables|Default|GetArrowBot)))
  (CallFunction|UpdateSelectorPosition))

(event EventInteract
  (params (HitComponent :type Primitive%20Component%20Object%20Reference))
  (bind _returnvalue (Game|GetPlayerController 0))
  ;[0.15 0.15 0.15 0.5] Enter in puzzle logic
  (Input|DisableInput (Game|GetPlayerCharacter 0) _returnvalue)
  (Game|Player|SetViewTargetwithBlend _returnvalue (Components|GetOwner (Variables|Default|GetCamera)) 0.4 "VTBlend_Linear" 0.0 false)
  (Input|EnableInput _returnvalue))

(event Input|KeyboardEvents|Q
  (params (Key :type Key%20Structure :default "None"))
  (bind _dialsvalue (Variables|Default|GetDialsValue))
  (bind _index (Variables|Default|GetIndex))
  (bind _output (Utilities|Array|Get(acopy) _dialsvalue _index))
  ;[0.15 0.15 0.15 0.5] Switch Values of dials
  (:Pressed
    (Variables|Default|SetForward? false)
    (if (not (Variables|Default|GetBusy))
      (Variables|Default|SetBusy true)
      (Utilities|Array|SetArrayElem _dialsvalue _index (Math|Integer|%(Integer) (+ (Math|Integer|%(Integer) (+ _output (Math|Integer|SelectInt 1 -1 (Variables|Default|GetForward?))) 10) 10) 10))
      (Development|PrintString (Utilities|String|Append "Molette" (Utilities|String|ToString(Integer) (Variables|Default|GetIndex)) "=" (Utilities|String|ToString(Integer) _output)) true true "(R=0.000000,G=0.660000,B=1.000000,A=1.000000)" 1e+03)
      (CallFunction|RotateDials (Variables|Default|GetForward?)))))

(event Input|KeyboardEvents|Z
  (params (Key :type Key%20Structure :default "None"))
  (bind _dials (Variables|Default|GetDials))
  ;[0.15 0.15 0.15 0.5] Switch Dials to rotate
  (:Pressed
    (if (not (Variables|Default|GetBusy))
      (if (Utilities|Array|IsValidIndex _dials (- (Variables|Default|GetIndex) 1))
        (Variables|Default|SetIndex (- (Variables|Default|GetIndex) 1))
        (else
          (Variables|Default|SetIndex (Utilities|Array|LastIndex _dials))))
      (CallFunction|UpdateSelectorPosition))))

(event Input|KeyboardEvents|S
  (params (Key :type Key%20Structure :default "None"))
  ;[0.15 0.15 0.15 0.5] Switch Dials to rotate
  (:Pressed
    (if (not (Variables|Default|GetBusy))
      (if (Utilities|Array|IsValidIndex (Variables|Default|GetDials) (+ (Variables|Default|GetIndex) 1))
        (Variables|Default|SetIndex (+ (Variables|Default|GetIndex) 1))
        (else
          (Variables|Default|SetIndex 0)))
      (CallFunction|UpdateSelectorPosition))))

(event Input|KeyboardEvents|D
  (params (Key :type Key%20Structure :default "None"))
  (bind _dialsvalue (Variables|Default|GetDialsValue))
  (bind _index (Variables|Default|GetIndex))
  (bind _output (Utilities|Array|Get(acopy) _dialsvalue _index))
  ;[0.15 0.15 0.15 0.5] Switch Values of dials
  (:Pressed
    (Variables|Default|SetForward? true)
    (if (not (Variables|Default|GetBusy))
      (Variables|Default|SetBusy true)
      (Utilities|Array|SetArrayElem _dialsvalue _index (Math|Integer|%(Integer) (+ (Math|Integer|%(Integer) (+ _output (Math|Integer|SelectInt 1 -1 (Variables|Default|GetForward?))) 10) 10) 10))
      (Development|PrintString (Utilities|String|Append "Molette" (Utilities|String|ToString(Integer) (Variables|Default|GetIndex)) "=" (Utilities|String|ToString(Integer) _output)) true true "(R=0.000000,G=0.660000,B=1.000000,A=1.000000)" 1e+03)
      (CallFunction|RotateDials (Variables|Default|GetForward?)))))

(event Input|KeyboardEvents|A
  (params (Key :type Key%20Structure :default "None"))
  (bind _returnvalue (Game|GetPlayerController 0))
  ;[0.15 0.15 0.15 0.5] Exit From Puzzle Logic
  (:Pressed
    ;;[0.15 0.15 0.15 0.5] Cast to the player to get camera
    (bind _asbp_first_person_character (Utilities|Casting|CastToBP_FirstPersonCharacter (Game|GetPlayerCharacter 0)))
    (Game|Player|SetViewTargetwithBlend _returnvalue (Components|GetOwner (Variables|/Game/FirstPerson/Blueprints/BP_FirstPersonCharacter.BP_FirstPersonCharacter_C|GetFirstPersonCamera _asbp_first_person_character)) 0.4 "VTBlend_Linear" 0.0 false)
    (Input|DisableInput _returnvalue)
    (Input|EnableInput (Game|GetPlayerCharacter 0) _returnvalue)))

(fn ConstructionScript)