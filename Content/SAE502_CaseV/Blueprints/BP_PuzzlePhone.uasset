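; BP_PuzzlePhone is a clickable phone keypad puzzle where the player enters a code of up to four characters to reveal hidden text actors.
; Every static mesh component gets click and hover bindings, with its first tag acting as the key value, Clear or Enter.
; Input updates the WBP_PhoneScreen widget.
; Enter compares it to RealCode, either solving the puzzle or briefly locking input with an error before resetting.
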(event Custom|ButtonHover
  (params (TouchedComponent :type Primitive%20Component%20Object%20Reference))
  ;[0.15 0.15 0.15 0.5] ButtonHover
  (if (not (== (Utilities|Array|Get(acopy) (Variables|/Script/Engine.ActorComponent|GetComponentTags TouchedComponent)) ""))
    (Variables|/Script/Engine.PlayerController|SetCurrentMouseCursor (Game|GetPlayerController 0) "Hand")))

(event Custom|OnButtonPressed
  (params (TouchedComponent :type Primitive%20Component%20Object%20Reference) (ButtonPressed :type Key%20Structure :default "None"))
  (bind _componenttags (Variables|/Script/Engine.ActorComponent|GetComponentTags TouchedComponent))
  (bind _output (Utilities|Array|Get(acopy) _componenttags))
  ;[0.15 0.15 0.15 0.5] OnButtonPressed
  (if (not (or (Variables|Default|GetbisInError) (Variables|Default|GetisSolved)))
    (if (not (== _output ""))
      (Audio|PlaySound2D "/Game/SAE502_CaseV/Audio/SFX/Phone/Button_press.Button_press" 1.0 (Math|Random|RandomFloatinRange 0.95 1.05) 0.0 "/Game/SAE502_CaseV/Audio/SFX/Phone/Phone_Concurrency.Phone_Concurrency" 0)
      (switch name _output
        (:Default
          (if (< (Utilities|String|Len (Variables|Default|GetCurrentCode)) 4)
            (Variables|Default|SetCurrentCode (Utilities|String|Append (Variables|Default|GetCurrentCode) (Utilities|String|ToString(Name) _output)))
            (bind _aswbp_phone_screen (Utilities|Casting|CastToWBP_PhoneScreen (UserInterface|GetUserWidgetObject (Variables|Default|GetPhoneScreen))))
            (Default|UpdateScreenText _aswbp_phone_screen (Variables|Default|GetCurrentCode))))
        (:Clear
          (CallFunction|ClearCode))
        (:Enter
          (CallFunction|ValidateCode))))))

(event Custom|ClearCode
  ;[0.15 0.15 0.15 0.5] ClearCode
  (Variables|Default|SetCurrentCode "")
  (bind _aswbp_phone_screen (Utilities|Casting|CastToWBP_PhoneScreen (UserInterface|GetUserWidgetObject (Variables|Default|GetPhoneScreen))))
  (Default|UpdateScreenText _aswbp_phone_screen (Variables|Default|GetCurrentCode)))

(event Custom|ValidateCode
  ;[0.15 0.15 0.15 0.5] ValidateCode
  (bind _aswbp_phone_screen (Utilities|Casting|CastToWBP_PhoneScreen (UserInterface|GetUserWidgetObject (Variables|Default|GetPhoneScreen))))
  (if (== (Variables|Default|GetCurrentCode) (Variables|Default|GetRealCode))
    (Audio|PlaySound2D "/Game/SAE502_CaseV/Audio/SFX/Phone/Right.Right" 1.0 1.0 0.0 "/Game/SAE502_CaseV/Audio/SFX/Phone/Phone_Concurrency.Phone_Concurrency" 0)
    (Variables|Default|SetisSolved true)
    (Default|UpdateScreenText _aswbp_phone_screen "OK")
    (for _array_element (Variables|Default|GetTextsActivated)
      (Rendering|SetActorHiddenInGame _array_element false))
    (else
      (Variables|Default|SetbisInError true)
      (Audio|PlaySound2D "/Game/SAE502_CaseV/Audio/SFX/Phone/Wrong.Wrong" 1.0 1.0 0.0 "/Game/SAE502_CaseV/Audio/SFX/Phone/Phone_Concurrency.Phone_Concurrency" 0)
      (Default|UpdateScreenText _aswbp_phone_screen "ERR")
      (Utilities|FlowControl|Delay 2.0)
      (Variables|Default|SetbisInError false)
      (Variables|Default|SetCurrentCode "")
      (Default|UpdateScreenText _aswbp_phone_screen "TAPEZ HELP"))))

(event Custom|EndButtonHover
  (params (TouchedComponent :type Primitive%20Component%20Object%20Reference))
  ;[0.15 0.15 0.15 0.5] EndButtonHover
  (if (not (== (Utilities|Array|Get(acopy) (Variables|/Script/Engine.ActorComponent|GetComponentTags TouchedComponent)) ""))
    (Variables|/Script/Engine.PlayerController|SetCurrentMouseCursor (Game|GetPlayerController 0) "Default")))

(event EventBeginPlay
  (|CallParentFunction)
  (for _array_element (Actor|GetComponentsByClass "/Script/Engine.StaticMeshComponent")
    ;[0.15 0.15 0.15 0.5] OnButtonPressed
    (EventDispatchers|BindEventtoOnClicked _array_element (delegate Custom|OnButtonPressed))
    ;[0.15 0.15 0.15 0.5] ButtonHover
    (EventDispatchers|BindEventtoOnBeginCursorOver _array_element (delegate Custom|ButtonHover))
    ;[0.15 0.15 0.15 0.5] EndButtonHover
    (EventDispatchers|BindEventtoOnEndCursorOver _array_element (delegate Custom|EndButtonHover))))

(event Collision|EventActorBeginOverlap
  (params (OtherActor :type Actor%20Object%20Reference))
  (|CallParentFunction OtherActor) ; This node is disabled and will not be called.\nDrag off pins to build functionality.
)

(event EventTick
  (params (DeltaSeconds :type Float%20%28single-precision%29))
  (|CallParentFunction DeltaSeconds) ; This node is disabled and will not be called.\nDrag off pins to build functionality.
)

(fn ConstructionScript
  (|CallParentFunction))