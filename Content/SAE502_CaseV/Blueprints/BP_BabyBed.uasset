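; BP_BabyBed is a bed that triggers a one-time horror scare when BP_Doll enters its detection zone.
; The overlap flags the doll as in bed, plays impact and laugh sounds, disables the zone, and flickers RedLight and SilhouetteDecal.
; The decal flickers through a self-rescheduling, randomly timed event.
; After a delay it fades and hides, but the cleared FlickerTimerHandle differs from the stored DecalTimeHandler, so the timer keeps running.
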(event OnComponentBeginOverlap(ZoneDetection)
  (params (OverlappedComponent :type Primitive%20Component%20Object%20Reference) (OtherActor :type Actor%20Object%20Reference) (OtherComp :type Primitive%20Component%20Object%20Reference) (OtherBodyIndex :type Integer) (bFromSweep :type Boolean) (SweepResult :type Hit%20Result%20Structure%20%28by%20ref%29))
  (bind _redlight (Variables|Default|GetRedLight))
  (bind _asbp_doll (Utilities|Casting|CastToBP_Doll OtherActor))
  (Utilities|FlowControl|DoOnce false
    (:Completed
      (Variables|/Game/SAE502_CaseV/Blueprints/BP_Doll.BP_Doll_C|SetbIsInBed _asbp_doll true)
      (Audio|PlaySound2D (Variables|Default|GetHorrorImpactSound) 1.0 1.0 0.0 0 0)
      (Default|PlayDollLaugh _asbp_doll)
      (Development|PrintString "La poupée est dans le lit")
      (Collision|SetCollisionEnabled (Variables|Default|GetZoneDetection) "NoCollision")
      (CallFunction|UpdateDecalFlicker)
      (Default|SetIsFlickering _redlight true)
      (Utilities|FlowControl|Delay 3.0)
      (Rendering|Components|Decal|SetFadeOut (Variables|/Script/Engine.DecalActor|GetDecal (Variables|Default|GetSilhouetteDecal)) 0.0 0.1 false)
      (Utilities|Time|ClearandInvalidateTimerbyHandle (Variables|Default|GetFlickerTimerHandle))
      (Default|SetIsFlickering _redlight false)
      (Rendering|SetActorHiddenInGame (Variables|Default|GetSilhouetteDecal) true))))

(event Custom|UpdateDecalFlicker
  (bind _silhouettedecal (Variables|Default|GetSilhouetteDecal))
  (if (> (Math|Random|RandomFloatinRange 0.0 1.0) 0.35)
    (Rendering|SetActorHiddenInGame _silhouettedecal false)
    (else
      (Rendering|SetActorHiddenInGame _silhouettedecal true)))
  (bind _returnvalue (Utilities|Time|SetTimerbyEvent (delegate Custom|UpdateDecalFlicker) (Math|Random|RandomFloatinRange 0.04 0.18)))
  (Variables|Default|SetDecalTimeHandler _returnvalue))

(event EventBeginPlay)

(event Collision|EventActorBeginOverlap
  (params (OtherActor :type Actor%20Object%20Reference)))

(event EventTick
  (params (DeltaSeconds :type Float%20%28single-precision%29)))

(fn ConstructionScript)