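; BP_Radio is an interactive radio prop that plays a list of music tracks over a white noise layer.
; Primary interact skips to the next track while on, and secondary interact toggles power, each with a pitch-randomized sound at the mesh.
; Tracks advance in a wrapping loop when audio finishes, with a manual-change flag around the delayed switch to keep Stop from triggering another skip.
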(event OnAudioFinished(Audio_Musique)
  ;[0.15 0.15 0.15 0.5] ChangeMusiqueOnfFinished
  (if (and (Variables|Default|GetbEstAllumee) (not (Variables|Default|GetbChangementManuel)))
    (CallFunction|MusiqueSuivante)))

(event Custom|JouerMusiqueActuelle
  (if (Variables|Default|GetbEstAllumee)
    (Audio|Components|Audio|SetSound (Variables|Default|GetAudio_Musique) (Utilities|Array|Get(acopy) (Variables|Default|GetListeMusiques) (Variables|Default|GetIndexMusiqueActuelle)))
    (Audio|Components|Audio|Play (Variables|Default|GetAudio_Musique) 0.0)
    (if (not (Audio|Components|Audio|IsPlaying (Variables|Default|GetAudio_WhiteNoise)))
      (Audio|Components|Audio|Play (Variables|Default|GetAudio_WhiteNoise) 0.0))))

(event Custom|MusiqueSuivante
  ;[0.15 0.15 0.15 0.5] Next music
  (Audio|PlaySoundatLocation (Variables|Default|GetSwitchSound) (Transformation|GetWorldLocation (Variables|Default|GetMesh)) "0, 0, 0" 1.0 (Math|Random|RandomFloatinRange 0.95 1.05) 0.0 (Variables|Default|GetSound_Attenuation) 0 0 0)
  (Variables|Default|SetbChangementManuel true)
  (Audio|Components|Audio|Stop (Variables|Default|GetAudio_Musique))
  (Utilities|FlowControl|Delay 0.2)
  (Variables|Default|SetIndexMusiqueActuelle (Math|Integer|%(Integer) (+ (Variables|Default|GetIndexMusiqueActuelle) 1) (Utilities|Array|Length (Variables|Default|GetListeMusiques))))
  (Variables|Default|SetbChangementManuel false)
  (CallFunction|JouerMusiqueActuelle))

(event Custom|ToggleRadio
  ;[0.15 0.15 0.15 0.5] ToggleRadio
  (Audio|PlaySoundatLocation (Variables|Default|GetToggleSound) (Transformation|GetWorldLocation (Variables|Default|GetMesh)) "0, 0, 0" 1.0 (Math|Random|RandomFloatinRange 0.95 1.05) 0.0 (Variables|Default|GetSound_Attenuation) 0 0 0)
  (bind _output_get (Variables|Default|SetbEstAllumee (not (Variables|Default|GetbEstAllumee))))
  (if _output_get
    (CallFunction|JouerMusiqueActuelle)
    (else
      (Variables|Default|SetbChangementManuel false)
      (Audio|Components|Audio|Stop (Variables|Default|GetAudio_Musique))
      (Audio|Components|Audio|Stop (Variables|Default|GetAudio_WhiteNoise))
      (Variables|Default|SetbChangementManuel true))))

(event EventBeginPlay
  (CallFunction|JouerMusiqueActuelle))

(event Collision|EventActorBeginOverlap
  (params (OtherActor :type Actor%20Object%20Reference)))

(event EventTick
  (params (DeltaSeconds :type Float%20%28single-precision%29)))

(event EventInteract
  (params (HitComponent :type Primitive%20Component%20Object%20Reference))
  (if (Variables|Default|GetbEstAllumee)
    (CallFunction|MusiqueSuivante)))

(event EventInteractSecondary
  (params (HitComponent :type Primitive%20Component%20Object%20Reference))
  (CallFunction|ToggleRadio))

(fn ConstructionScript)