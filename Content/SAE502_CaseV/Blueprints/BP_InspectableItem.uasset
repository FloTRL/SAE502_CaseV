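; BP_InspectableItem is an interactable item that the player can pick up to examine in a separate inspection view.
; On Interact it plays a pickup sound and copies its mesh, scale, first material and configured initial rotation onto the level's BP_InspectViewer.
; It then opens a WBP_InspectOverlay widget linked to the viewer and itself.
; OnInspectionClosed is an empty hook in this Blueprint.
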(event Custom|OnInspectionClosed)

(event EventInteract
  (params (HitComponent :type Primitive%20Component%20Object%20Reference))
  (bind _inspectableitemmesh (Variables|Default|GetInspectableItemMesh))
  (Audio|PlaySound2D (Variables|Default|GetPickUpSound) 1.0 1.0 0.0 0 0)
  (bind _returnvalue (Actor|GetActorOfClass "/Game/SAE502_CaseV/Blueprints/BP_InspectViewer.BP_InspectViewer_C"))
  (Components|StaticMesh|SetStaticMesh (Variables|/Game/SAE502_CaseV/Blueprints/BP_InspectViewer.BP_InspectViewer_C|GetInspectedMesh _returnvalue) (Variables|/Script/Engine.StaticMeshComponent|GetStaticMesh _inspectableitemmesh))
  (Transformation|SetWorldScale3D (Variables|/Game/SAE502_CaseV/Blueprints/BP_InspectViewer.BP_InspectViewer_C|GetInspectedMesh _returnvalue) (Transformation|GetWorldScale _inspectableitemmesh))
  (Rendering|Material|SetMaterial (Variables|/Game/SAE502_CaseV/Blueprints/BP_InspectViewer.BP_InspectViewer_C|GetInspectedMesh _returnvalue) 0 (Rendering|Material|GetMaterial _inspectableitemmesh 0))
  (Transformation|SetRelativeRotation (Variables|/Game/SAE502_CaseV/Blueprints/BP_InspectViewer.BP_InspectViewer_C|GetInspectedMesh _returnvalue) (Variables|Default|GetInspectionInitialRotation) false false)
  (bind _returnvalue_2 (UserInterface|CreateWidget "/Game/SAE502_CaseV/Blueprints/WBP_InspectOverlay.WBP_InspectOverlay_C" 0 _returnvalue self))
  (UserInterface|Viewport|AddtoViewport _returnvalue_2 0))

(fn ConstructionScript)