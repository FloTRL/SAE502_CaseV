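; BP_Doll is a grabbable doll that plays laughter through its VoiceAudio component.
; It extends the parent's grab and drop events, fading in a laugh on grab unless IsInBed is set and fading the audio out on drop.
; A separate PlayDollLaugh event stops the current sound and immediately plays a softer laugh.
; IsInBed is only read here, never set.
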(event Custom|PlayDollLaugh
  (Audio|Components|Audio|Stop (Variables|Default|GetVoiceAudio))
  (Audio|Components|Audio|SetSound (Variables|Default|GetVoiceAudio) (Variables|Default|GetSoftLaughSound))
  (Audio|Components|Audio|Play (Variables|Default|GetVoiceAudio) 0.0))

(event EventBeginPlay
  (|CallParentFunction) ; This node is disabled and will not be called.\nDrag off pins to build functionality.
)

(event Collision|EventActorBeginOverlap
  (params (OtherActor :type Actor%20Object%20Reference))
  (|CallParentFunction OtherActor) ; This node is disabled and will not be called.\nDrag off pins to build functionality.
)

(event EventTick
  (params (DeltaSeconds :type Float%20%28single-precision%29))
  (|CallParentFunction DeltaSeconds) ; This node is disabled and will not be called.\nDrag off pins to build functionality.
)

(event EventOnGrab
  (params (GrabbedComponent :type Primitive%20Component%20Object%20Reference))
  (bind _voiceaudio (Variables|Default|GetVoiceAudio))
  (|CallParentFunction GrabbedComponent)
  (if (not (Variables|Default|GetbIsInBed))
    (Audio|Components|Audio|SetSound _voiceaudio (Variables|Default|GetLaughSound))
    (Audio|Components|Audio|FadeIn _voiceaudio 0.5 1.0 0.0 "Linear" :!class /Script/Engine.AudioComponent)))

(event EventOnDrop
  (params (Grabbed%20Componenet :type Primitive%20Component%20Object%20Reference))
  (|CallParentFunction Grabbed%20Componenet)
  (Audio|Components|Audio|FadeOut (Variables|Default|GetVoiceAudio) 0.25 0.0 "Linear" :!class /Script/Engine.AudioComponent))

(fn ConstructionScript
  (|CallParentFunction))