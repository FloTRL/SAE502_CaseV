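; Base door actor that the player can unlock, open and close through its Interact event.
; It unlocks when an optional linked padlock fires its opened event, or by consuming the required key from the first-person character's inventory.
; Once unlocked, a Timeline swings the door's yaw forward or in reverse, with a busy flag blocking re-triggering.
; Sounds accompany movement, slamming and key unlocking, while printed French messages report key results.
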(event Custom|DebloquerPorte
  (Variables|Default|SetbisUnlocked true))

(event EventBeginPlay
  (bind _cadenasassocie (Variables|Default|GetcadenasAssocie))
  (Utilities|IsValid _cadenasassocie
    (:Is%20Valid
      (EventDispatchers|BindEventtoOnCadenasOuvert _cadenasassocie (delegate Custom|DebloquerPorte)))))

(event Collision|EventActorBeginOverlap
  (params (OtherActor :type Actor%20Object%20Reference)))

(event EventTick
  (params (DeltaSeconds :type Float%20%28single-precision%29)))

(event EventInteract
  (params (HitComponent :type Primitive%20Component%20Object%20Reference))
  (bind _returnvalue (Transformation|GetActorLocation))
  (if (Variables|Default|GetbisUnlocked)
    (if (not (Variables|Default|GetbisBusy))
      (if (Variables|Default|GetbisOpen)
        (Variables|Default|SetbisBusy true)
        (Audio|PlaySoundatLocation "/Game/SAE502_CaseV/Audio/SFX/DOOR/RENDER/CLOSING/DOOR_CLOSING.DOOR_CLOSING" _returnvalue "0, 0, 0" 1.0 1.0 0.0 0 0 0 0)
        (bind _doorrotation (Timeline|Timeline ReverseFromEnd)
          (:Update
            (Transformation|SetRelativeRotation (Variables|Default|GetDoor) (Math|Rotator|MakeRotator 0.0 0.0 _doorrotation) false false))
          (:Finished
            (Variables|Default|SetbisOpen (not (Variables|Default|GetbisOpen)))
            (Variables|Default|SetbisBusy (not (Variables|Default|GetbisBusy)))
            (if (not (Variables|Default|GetbisOpen))
              (Audio|PlaySoundatLocation "/Game/SAE502_CaseV/Audio/SFX/DOOR/RENDER/SLAM/DOOR_SLAM.DOOR_SLAM" (Transformation|GetActorLocation) "0, 0, 0" 1.0 1.0 0.0 0 0 0 0))))
        (else
          (Variables|Default|SetbisBusy true)
          (Audio|PlaySoundatLocation "/Game/SAE502_CaseV/Audio/SFX/DOOR/RENDER/OPENING/DOOR_OPENING.DOOR_OPENING" _returnvalue "0, 0, 0" 1.0 1.0 0.0 0 0 0 0)
          (Timeline|Timeline PlayFromStart))))
    (else
      (bind _asbp_first_person_character (Utilities|Casting|CastToBP_FirstPersonCharacter (Game|GetPlayerCharacter 0)))
      (if (Utilities|Array|ContainsItem (Variables|/Game/FirstPerson/Blueprints/BP_FirstPersonCharacter.BP_FirstPersonCharacter_C|GetInventoryKeys _asbp_first_person_character) (Variables|Default|GetRequiredKey))
        (Variables|Default|SetbisUnlocked true)
        (Development|PrintString "Porte Déverouillée !")
        (Utilities|Array|RemoveItem (Variables|/Game/FirstPerson/Blueprints/BP_FirstPersonCharacter.BP_FirstPersonCharacter_C|GetInventoryKeys _asbp_first_person_character) (Variables|Default|GetRequiredKey))
        (Audio|PlaySoundatLocation "/Game/SAE502_CaseV/Audio/SFX/DOOR/RENDER/UNLOCK/DOOR_UNLOCK.DOOR_UNLOCK" (Transformation|GetActorLocation) "0, 0, 0" 1.0 1.0 0.0 0 0 0 0)
        (else
          (Development|PrintString "La porte est vérouillée"))))))

(fn ConstructionScript)