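; Base lamp actor that can be switched on and off, flicker, or break, with matching audio.
; Construction caches every light component's intensity and the "bulb"-tagged mesh's emissive value via a dynamic material, so one multiplier scales both.
; SetLightState drives that multiplier, using a looping timer for random flicker dips.
; Interact toggles directly interactable lamps, while BreakLight runs once, flickering before going permanently dark after a delay.
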(event Custom|FlickerUpdate
  (bind _output_get (Variables|Default|SetcurrentFlickerMultiplier (Math|Float|SelectFloat 1.0 0.05 (Math|Random|RandomBoolwithWeight 0.85))))
  (CallFunction|ApplyLightsMultiplier _output_get))

(event Custom|BreakLight
  (Utilities|FlowControl|DoOnce false
    (:Completed
      (CallFunction|SetIsFlickering true)
      (CallFunction|SetLightState (Variables|Default|GetbisOn))
      (Utilities|FlowControl|Delay (Variables|Default|GetbreakDelay))
      (Variables|Default|SetbisBroken true)
      (Variables|Default|SetbisOn true)
      (Utilities|Time|ClearandInvalidateTimerbyHandle (Variables|Default|GetFlickerTimeHandler))
      (Audio|Components|Audio|Stop (Variables|Default|GetFlickeringAudio))
      (CallFunction|ApplyLightsMultiplier 0.0)
      (Audio|PlaySoundatLocation (Variables|Default|GetbreakSound) (Transformation|GetActorLocation) "0, 0, 0" 1.0 (Math|Random|RandomFloatinRange 0.95 1.05) 0.0 (Variables|Default|GetSoundAttenuation) 0 0 0))))

(event EventBeginPlay
  (CallFunction|SetLightState (Variables|Default|GetbisOn)))

(event Collision|EventActorBeginOverlap
  (params (OtherActor :type Actor%20Object%20Reference)))

(event EventTick
  (params (DeltaSeconds :type Float%20%28single-precision%29)))

(event EventSetLightState
  (params (bisOn :type Boolean))
  (if (Variables|Default|GetbisBroken)
    (Variables|Default|SetbisOn false)
    (else
      (bind _output_get (Variables|Default|SetbisOn bisOn))
      (if _output_get
        (if (Variables|Default|GetbisFlickering)
          (bind _returnvalue (Utilities|Time|SetTimerbyEvent (delegate Custom|FlickerUpdate) 0.1 true))
          (Variables|Default|SetFlickerTimeHandler _returnvalue)
          (Audio|Components|Audio|Play (Variables|Default|GetFlickeringAudio) 0.0)
          (else
            (CallFunction|ApplyLightsMultiplier 1.0)
            (Audio|Components|Audio|Stop (Variables|Default|GetFlickeringAudio))))
        (else
          (Audio|Components|Audio|Stop (Variables|Default|GetFlickeringAudio))
          (Utilities|Time|ClearandInvalidateTimerbyHandle (Variables|Default|GetFlickerTimeHandler))
          (CallFunction|ApplyLightsMultiplier 0.0))))))

(event EventInteract
  (params (HitComponent :type Primitive%20Component%20Object%20Reference))
  (bind _returnvalue (Transformation|GetActorLocation))
  (bind _returnvalue_2 (Math|Random|RandomFloatinRange 0.95 1.05))
  (bind _soundattenuation (Variables|Default|GetSoundAttenuation))
  (if (Variables|Default|GetbIsDirectlyInteractable)
    (if (Variables|Default|GetbisOn)
      (Audio|PlaySoundatLocation (Variables|Default|GetSelfSwitchOffSound) _returnvalue "0, 0, 0" 1.0 _returnvalue_2 0.0 _soundattenuation 0 0 0)
      (else
        (Audio|PlaySoundatLocation (Variables|Default|GetSelfSwitchOnSound) _returnvalue "0, 0, 0" 1.0 _returnvalue_2 0.0 _soundattenuation 0 0 0)))
    (CallFunction|SetLightState (not (Variables|Default|GetbisOn)))))

(fn ConstructionScript
  (bind _returnvalue (Actor|GetComponentsbyTag "/Script/Engine.StaticMeshComponent" "bulb"))
  (bind _output (Utilities|Array|Get(acopy) _returnvalue))
  (Utilities|Array|Clear (Variables|Default|GetLightComponents))
  (Utilities|Array|Clear (Variables|Default|GetBaseIntensities))
  (for _array_element (Actor|GetComponentsByClass "/Script/Engine.LightComponent")
    (Utilities|Array|Add (Variables|Default|GetLightComponents) _array_element)
    (Utilities|Array|Add (Variables|Default|GetBaseIntensities) (Variables|/Script/Engine.LightComponentBase|GetIntensity _array_element)))
  (Utilities|IsValid _output
    (:Is%20Valid
      (bind _returnvalue_2 (Rendering|Material|CreateDynamicMaterialInstance _output 0 0 "None" :!class /Script/Engine.PrimitiveComponent))
      (bind _output_get (Variables|Default|SetBulbInMat _returnvalue_2))
      (bind _returnvalue_3 (Rendering|Material|GetScalarParameterValue _output_get "EmissiveIntensity" :!class /Script/Engine.MaterialInstanceDynamic))
      (Variables|Default|SetBaseEmissiveIntensity _returnvalue_3))
    (:Is%20Not%20Valid
      (Variables|Default|SetBulbInMat 0))))

(fn ApplyLightsMultiplier
  (params (Multiplier :type Float%20%28double-precision%29))
  (for (_array_element _array_index) (Variables|Default|GetLightComponents)
    (Rendering|Components|Light|SetIntensity _array_element (* Multiplier (Utilities|Array|Get(acopy) (Variables|Default|GetBaseIntensities) _array_index))))
  (if (Utilities|IsValid (Variables|Default|GetBulbInMat))
    (Rendering|Material|SetScalarParameterValue (Variables|Default|GetBulbInMat) "EmissiveIntensity" (* Multiplier (Variables|Default|GetBaseEmissiveIntensity)) :!class /Script/Engine.MaterialInstanceDynamic)))

(fn SetIsFlickering
  (params (bEnable :type Boolean))
  (bind _output_get (Variables|Default|SetbisFlickering bEnable))
  (if _output_get
    (CallFunction|SetLightState (Variables|Default|GetbisOn))
    (else
      (Utilities|Time|ClearandInvalidateTimerbyHandle (Variables|Default|GetFlickerTimeHandler)))))