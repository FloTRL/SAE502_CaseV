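; Monster enemy character that screams at a sighted pawn, hunts it through a Behavior Tree and attacks in melee.
; First sighting via PawnSensing turns it, plays the scream montage, then writes the pawn to the TargetPlayer blackboard key.
; Point damage instead targets the damage causer immediately and plays bone-specific hit reactions.
; LancerAttaque plays the attack montage, while DeclencherCoup applies damage through a forward sphere trace with debug drawing.
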(event OnSeePawn(PawnSensing)
  (params (Pawn :type Pawn%20Object%20Reference))
  (if (not (Variables|Default|GetbisChasing))
    (Utilities|FlowControl|DoOnce false
      (:Completed
        (Transformation|SetActorRotation (Math|Rotator|MakeRotator 0.0 0.0 (.yaw (Math|Rotator|FindLookatRotation (Transformation|GetActorLocation) (Transformation|GetActorLocation Pawn)))))
        (Class|NavMovementInterface|StopActiveMovement (Variables|Character|GetCharacterMovement))
        (Animation|Montage|PlayMontage (Variables|Character|GetMesh) "/Game/SAE502_CaseV/Animation/AM_Monster_Scream.AM_Monster_Scream"
          (:OnCompleted
            ;[0.15 0.15 0.15 0.5] Start BT
            (AI|Components|Blackboard|SetValueasObject (AI|GetBlackboard (AI|GetAIController self)) (Utilities|Name|MakeLiteralName "TargetPlayer") Pawn)))))))

(event Custom|Lancer%20Attaque
  (Class|NavMovementInterface|StopActiveMovement (Variables|Character|GetCharacterMovement))
  (Animation|PlayAnimMontage "/Game/SAE502_CaseV/Animation/AM_Zombie_Attack_1__Anim.AM_Zombie_Attack_1__Anim" 1.25 "None"))

(event Custom|DeclencherCoup
  (bind _returnvalue (Transformation|GetActorLocation))
  (bind (_outhit _returnvalue_2) (Collision|SphereTraceByChannel _returnvalue (+ _returnvalue (* (Math|Vector|GetForwardVector (Variables|Collision|GetCapsuleComponent)) "120.000000,120.000000,120.000000")) 4e+01 "TraceTypeQuery1" false 0 "ForDuration"))
  (if _returnvalue_2
    (Game|Damage|ApplyDamage (.HitActor (Collision|BreakHitResult _outhit)) 1e+01 0 0)))

(event EventBeginPlay)

(event Collision|EventActorBeginOverlap
  (params (OtherActor :type Actor%20Object%20Reference)))

(event EventTick
  (params (DeltaSeconds :type Float%20%28single-precision%29)))

(event Game|Damage|EventPointDamage
  (params (Damage :type Float%20%28single-precision%29) (DamageType :type Damage%20Type%20Object%20Reference) (HitLocation :type Vector :default "0, 0, 0") (HitNormal :type Vector :default "0, 0, 0") (HitComponent :type Primitive%20Component%20Object%20Reference) (BoneName :type Name :default "None") (ShotFromDirection :type Vector :default "0, 0, 0") (InstigatedBy :type Controller%20Object%20Reference) (DamageCauser :type Actor%20Object%20Reference) (HitInfo :type Hit%20Result%20Structure%20%28by%20ref%29))
  (Variables|Default|SetbisChasing true)
  ;[0.15 0.15 0.15 0.5] Start BT
  (AI|Components|Blackboard|SetValueasObject (AI|GetBlackboard (AI|GetAIController self)) (Utilities|Name|MakeLiteralName "TargetPlayer") DamageCauser)
  (switch name BoneName
    (:head
      (Animation|Montage|PlayMontage (Variables|Character|GetMesh) "/Game/SAE502_CaseV/Animation/AM_Degat_Tete.AM_Degat_Tete"))
    (:clavicle_r
      (Animation|Montage|PlayMontage (Variables|Character|GetMesh) "/Game/SAE502_CaseV/Animation/AM_Monster_Degat_ClavicleL.AM_Monster_Degat_ClavicleL" :!label _label))
    (:upperarm_r
      (goto _label))
    (:lowerarm_r
      (goto _label))
    (:clavicle_l
      (Animation|Montage|PlayMontage (Variables|Character|GetMesh) "/Game/SAE502_CaseV/Animation/AM_Monster_Degat_ClavicleR.AM_Monster_Degat_ClavicleR" :!label _label_2))
    (:upperarm_l
      (goto _label_2))
    (:lowerarm_l
      (goto _label_2))))

(fn ConstructionScript)