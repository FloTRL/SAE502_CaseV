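; Base Blueprint for pickup props that can be grabbed and thrown.
; ThrowObject adds a fixed linear velocity to the target component along the player camera's forward vector.
; OnGrab snaps the audio component onto the grabbed component, plays the carry sound and prints a debug message.
; OnDrop is an empty event, so nothing here stops the carry sound.
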(event EventBeginPlay)

(event Collision|EventActorBeginOverlap
  (params (OtherActor :type Actor%20Object%20Reference)))

(event EventTick
  (params (DeltaSeconds :type Float%20%28single-precision%29)))

(event EventThrowObject
  (params (TargetComponent :type Primitive%20Component%20Object%20Reference))
  ;[0.15 0.15 0.15 0.5] ThrowObject
  (Physics|SetPhysicsLinearVelocity TargetComponent (* (Math|Vector|GetForwardVector (Camera|GetCameraRotation (Variables|/Script/Engine.PlayerController|GetPlayerCameraManager (Game|GetPlayerController 0)))) 5e+02) true "None"))

(event EventOnGrab
  (params (GrabbedComponent :type Primitive%20Component%20Object%20Reference))
  (bind _audio (Variables|Default|GetAudio))
  (Transformation|AttachComponentToComponent (Variables|Default|GetAudio) GrabbedComponent "None" "SnapToTarget" "KeepRelative" "KeepRelative" true)
  (Development|PrintString "Grabbed")
  (Audio|Components|Audio|SetSound _audio (Variables|Default|GetCarrySound))
  (Audio|Components|Audio|Play _audio 0.0))

(event EventOnDrop
  (params (Grabbed%20Componenet :type Primitive%20Component%20Object%20Reference)))

(fn ConstructionScript)