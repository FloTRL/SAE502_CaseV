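; BP_PuzzleItem is an interactable puzzle actor that moves the player from first-person control into a fixed-camera, mouse-driven puzzle view and back.
; Interact disables character input, blends the view to the actor's own camera, enables cursor, click and hover events, and takes input itself.
; Exit, also triggered by the A key, blends back to the first-person character and restores game-only input.
; The file holds only this view and input switching, with no puzzle-solving logic.
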(event Custom|Exit
  (bind _returnvalue (Game|GetPlayerController 0))
  (bind _returnvalue_2 (Game|GetPlayerController 0))
  ;[0.15 0.15 0.15 0.5] Exit From Puzzle Logic
  ;;[0.15 0.15 0.15 0.5] Cast to the player to get camera
  (bind _asbp_first_person_character (Utilities|Casting|CastToBP_FirstPersonCharacter (Game|GetPlayerCharacter 0)))
  (Game|Player|SetViewTargetwithBlend _returnvalue (Components|GetOwner (Variables|/Game/FirstPerson/Blueprints/BP_FirstPersonCharacter.BP_FirstPersonCharacter_C|GetFirstPersonCamera _asbp_first_person_character)) 0.4 "VTBlend_Linear" 0.0 false)
  (Input|DisableInput _returnvalue)
  (Input|EnableInput (Game|GetPlayerCharacter 0) _returnvalue)
  (Input|SetInputModeGameOnly _returnvalue_2 false)
  (Variables|/Script/Engine.PlayerController|SetbShowMouseCursor _returnvalue_2 false)
  (Variables|/Script/Engine.PlayerController|SetbEnableClickEvents _returnvalue_2 false)
  (Variables|/Script/Engine.PlayerController|SetbEnableMouseOverEvents _returnvalue_2 false))

(event EventBeginPlay)

(event Collision|EventActorBeginOverlap
  (params (OtherActor :type Actor%20Object%20Reference)))

(event EventTick
  (params (DeltaSeconds :type Float%20%28single-precision%29)))

(event EventInteract
  (bind _returnvalue (Game|GetPlayerController 0))
  (bind _returnvalue_2 (Game|GetPlayerController 0))
  ;[0.15 0.15 0.15 0.5] Enter in puzzle logic
  (Input|DisableInput (Game|GetPlayerCharacter 0) _returnvalue)
  (Game|Player|SetViewTargetwithBlend _returnvalue (Components|GetOwner (Variables|Default|GetCamera)) 0.4 "VTBlend_Linear" 0.0 false)
  (Variables|/Script/Engine.PlayerController|SetbShowMouseCursor _returnvalue_2 true)
  (Variables|/Script/Engine.PlayerController|SetbEnableClickEvents _returnvalue_2 true)
  (Variables|/Script/Engine.PlayerController|SetbEnableMouseOverEvents _returnvalue_2 true)
  (Input|SetInputModeGameandUI _returnvalue_2 0 "DoNotLock" false false)
  (Input|EnableInput _returnvalue))

(event Input|KeyboardEvents|A
  (params (Key :type Key%20Structure :default "None"))
  (bind _returnvalue (Game|GetPlayerController 0))
  (bind _returnvalue_2 (Game|GetPlayerController 0))
  ;[0.15 0.15 0.15 0.5] Exit From Puzzle Logic
  (:Pressed
    ;;[0.15 0.15 0.15 0.5] Cast to the player to get camera
    (bind _asbp_first_person_character (Utilities|Casting|CastToBP_FirstPersonCharacter (Game|GetPlayerCharacter 0)))
    (Game|Player|SetViewTargetwithBlend _returnvalue (Components|GetOwner (Variables|/Game/FirstPerson/Blueprints/BP_FirstPersonCharacter.BP_FirstPersonCharacter_C|GetFirstPersonCamera _asbp_first_person_character)) 0.4 "VTBlend_Linear" 0.0 false)
    (Input|DisableInput _returnvalue)
    (Input|EnableInput (Game|GetPlayerCharacter 0) _returnvalue)
    (Input|SetInputModeGameOnly _returnvalue_2 false)
    (Variables|/Script/Engine.PlayerController|SetbShowMouseCursor _returnvalue_2 false)
    (Variables|/Script/Engine.PlayerController|SetbEnableClickEvents _returnvalue_2 false)
    (Variables|/Script/Engine.PlayerController|SetbEnableMouseOverEvents _returnvalue_2 false)))

(fn ConstructionScript)