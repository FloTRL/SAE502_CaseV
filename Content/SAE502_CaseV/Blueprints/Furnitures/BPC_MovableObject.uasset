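; BPC_MovableObject is a component for furniture parts that toggles between a closed pose and an open pose offset in location and rotation.
; ToggleElement flips the state, plays the matching open or close sound, sets the target relative transform and enables tick.
; Tick interpolates location and rotation toward that target, then snaps and disables itself when within tolerance, so it only ticks while moving.
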(event EventBeginPlay
  (Components|Tick|SetComponentTickEnabled false)
  (bind _output_get (Variables|Default|SetInitialRelativeTransform (Transformation|GetRelativeTransform)))
  (Variables|Default|SetTargetRelativeTransform _output_get))

(event EventTick
  (params (DeltaSeconds :type Float%20%28single-precision%29))
  (bind _returnvalue (Transformation|GetRelativeTransform))
  (bind _targetrelativetransform (Variables|Default|GetTargetRelativeTransform))
  (bind _interpspeed (Variables|Default|GetInterpSpeed))
  (Transformation|SetRelativeLocationAndRotation (Math|Interpolation|VInterpTo (.location _returnvalue) (.location _targetrelativetransform) DeltaSeconds _interpspeed) (Math|Interpolation|RInterpTo (.rotation _returnvalue) (.rotation _targetrelativetransform) DeltaSeconds _interpspeed) false false)
  (if (and (Utilities|Operators|EqualEqual (Variables|Default|GetRelativeLocation) (.location _targetrelativetransform) 0.1) (Utilities|Operators|EqualEqual (Variables|Default|GetRelativeRotation) (.rotation _targetrelativetransform) 0.1))
    (Transformation|SetRelativeTransform (Variables|Default|GetTargetRelativeTransform) false false)
    (Components|Tick|SetComponentTickEnabled false)))

(fn ToggleElement
  (bind _returnvalue (Transformation|GetWorldLocation))
  (bind _soundattenuation (Variables|Default|GetSoundAttenuation))
  (bind _output_get (Variables|Default|SetbisOpen (not (Variables|Default|GetbisOpen))))
  (if _output_get
    (Audio|PlaySoundatLocation (Variables|Default|GetOpenSound) _returnvalue "0, 0, 0" 1.0 1.0 0.0 _soundattenuation 0 0 0)
    (Variables|Default|SetTargetRelativeTransform (Math|Transform|MakeTransform (+ (.location (Variables|Default|GetTargetRelativeTransform)) (Variables|Default|GetTargetOffsetLocation)) (Math|Rotator|CombineRotators (.rotation (Variables|Default|GetTargetRelativeTransform)) (Variables|Default|GetTargetOffsetRotation)) (.scale (Variables|Default|GetTargetRelativeTransform))))
    (else
      (Audio|PlaySoundatLocation (Variables|Default|GetCloseSound) _returnvalue "0, 0, 0" 1.0 1.0 0.0 _soundattenuation 0 0 0)
      (Variables|Default|SetTargetRelativeTransform (Variables|Default|GetInitialRelativeTransform))))
  (Components|Tick|SetComponentTickEnabled true))